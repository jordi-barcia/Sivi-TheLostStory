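; Waterfall smoke volume actor that sets up a Niagara-driven fog effect in its construction script, with a debug box matching the volume size.
; A dynamic smoke material receives shape type and volume size, then feeds the NSFogWrite Niagara component.
; A downward orthographic scene capture renders selected height actors into FogHeightRT.
; Most other material parameters, including height texture and method, are unwired, and the event graph is empty.
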(fn `CaptureHeight`
  (`SceneCaptureComponent2D.CaptureScene` (`self.HeightCapture`))
  (return))

(fn `HeightCaptureSetup`
  (locals (NewLocalVarNewLocalVar :type "TextureParameterValue Structure"))
  (bind (_returnvalue_x _returnvalue_y _returnvalue_z) (`KismetMathLibrary.BreakVector` (`self.K2_GetActorLocation`)))
  (bind (_volumesize_x _volumesize_y _volumesize_z) (`KismetMathLibrary.BreakVector` (`self.VolumeSize`)))
  (bind _heightcapture (`self.HeightCapture`))
  (bind (_volumesize_x_2 _volumesize_y_2 _volumesize_z_2) (`KismetMathLibrary.BreakVector` (`self.VolumeSize`)))
  (`SceneComponent.K2_SetWorldLocationAndRotation` _heightcapture (`KismetMathLibrary.MakeVector` _returnvalue_x _returnvalue_y (/ _returnvalue_z (/ _volumesize_z_2 2.0))) (struct :`Pitch` -90.0 :`Roll` -90.0) false false)
  (set `SceneCaptureComponent2D.OrthoWidth` (`KismetMathLibrary.FMax` (`KismetMathLibrary.FMax` _volumesize_x _volumesize_y) _volumesize_z) _heightcapture)
  (set `SceneCaptureComponent2D.TextureTarget` (`self.FogHeightRT`) _heightcapture)
  (set `SceneCaptureComponent.ShowOnlyActors` (`self.HeightActors`) _heightcapture)
  (`self.CaptureHeight`))

(fn `Set Fog MID variables`
  (bind _fog_mid (`self.Fog MID`))
  (`MaterialInstanceDynamic.SetVectorParameterValue` _fog_mid "ShapeType" (select `/Game/VFX/VL_Fog/E_FogShapeType` (`self.ShapeType`) :`NewEnumerator0` (struct :`B` 1.0) :`NewEnumerator1` (struct :`A` 1.0) :`NewEnumerator2` (struct :`G` 1.0) :`NewEnumerator3` (struct :`R` 1.0) :!type "LinearColor Structure"))
  (`MaterialInstanceDynamic.SetVectorParameterValue` _fog_mid "VolumeSize" (`KismetMathLibrary.Conv_VectorToLinearColor` (`self.VolumeSize`))))

(fn `Set Niagara Variables`
  (bind _ns_fogwrite (`self.NS_FogWrite`))
  (bind (_volumesize_x _volumesize_y _volumesize_z) (`KismetMathLibrary.BreakVector` (`self.VolumeSize`)))
  (`NiagaraComponent.SetVariableMaterial` _ns_fogwrite "FogMID" (`self.Fog MID`))
  (`NiagaraComponent.SetVariableFloat` _ns_fogwrite "VolumeSizeMax" (* (`KismetMathLibrary.FMax` (`KismetMathLibrary.FMax` _volumesize_x _volumesize_y) _volumesize_z) 2.0))
  (return))

(fn `UserConstructionScript`
  (bind _returnvalue (`KismetMaterialLibrary.CreateDynamicMaterialInstance` "/Game/VFX/VL_Fog/VL_WaterfallSmokeMaterial.VL_WaterfallSmokeMaterial"))
  (set `self.Fog MID` _returnvalue)
  (`KismetRenderingLibrary.CreateRenderTarget2D` 256 256 "RTF_RG32f")
  (`BoxComponent.SetBoxExtent` (`self.DebugBox`) (/ (`self.VolumeSize`) 2.0) true)
  (`self.Set Niagara Variables`)
  (`self.Set Fog MID variables`)
  (`self.HeightCaptureSetup`))